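; Test actor that tethers a spawned, physics-simulated Manny head mesh to the skeletal mesh's right upper-arm socket.
; On BeginPlay it spawns the movable static mesh actor and adds linear damping to the skeletal mesh.
; A runtime-added cable component draws the tether between socket and mesh.
; A runtime physics constraint links bone and mesh, with locked swing, limited twist and limited X and Z travel.
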(event EventBeginPlay
  (bind _skeletalmesh (Variables|Default|GetSkeletalMesh))
  (bind _skeletalmesh_2 (Variables|Default|GetSkeletalMesh))
  (bind _returnvalue (Transformation|GetSocketTransform _skeletalmesh_2 "upperarm_r" "RTS_World"))
  (bind (_location _rotation _scale) (Math|Transform|BreakTransform _returnvalue))
  (Utilities|FlowControl|Sequence
    (:then_0
      ;[1 1 1] Spawn Mesh
      (bind _returnvalue_2 (Game|SpawnActorfromClass "/Script/Engine.StaticMeshActor" _returnvalue "Undefined" "MultiplyWithRoot" 0 0))
      (bind _output_get (Variables|Default|SetMyMeshSpawned _returnvalue_2))
      (Components|StaticMesh|SetStaticMesh (Variables|/Script/Engine.StaticMeshActor|GetStaticMeshComponent _returnvalue_2) "/Game/Characters/UE4_MannySplit/UE4_Manny_Head.UE4_Manny_Head")
      (Class|PrimitiveComponent|SetLinearDamping _skeletalmesh 6.0)
      (Collision|SetCollisionProfileName _skeletalmesh "PhysicsActor" true :!class /Script/Engine.PrimitiveComponent)
      (Transformation|SetMobility _output_get "Movable")
      (Physics|SetSimulatePhysics (Variables|/Script/Engine.StaticMeshActor|GetStaticMeshComponent _returnvalue_2) true))
    (:then_1
      ;[1 1 1] Setup Cable Component
      (bind _returnvalue_3 (AddComponent|AddCableComponent true _returnvalue))
      (bind _output_get_2 (Variables|Default|SetCableComp _returnvalue_3))
      (Transformation|AttachComponentToComponent _returnvalue_3 (Variables|Default|GetSkeletalMesh) "upperarm_r" "SnapToTarget" "KeepRelative" "KeepRelative" true)
      (Variables|/Script/CableComponent.CableComponent|SetEndLocation _output_get_2 "0, 0, 0")
      (Variables|/Script/CableComponent.CableComponent|SetCableWidth _output_get_2 4.5)
      (Variables|/Script/CableComponent.CableComponent|SetCableLength _output_get_2 2e+01)
      (Class|CableComponent|SetAttachEndtoComponent _returnvalue_3 (Variables|/Script/Engine.StaticMeshActor|GetStaticMeshComponent (Variables|Default|GetMyMeshSpawned)) "Pivot"))
    (:then_2
      ;[1 1 1] Setup Phyics
      (bind _returnvalue_4 (AddComponent|AddPhysicsConstraintComponent true (Math|Transform|MakeTransform _location (Transformation|GetActorRotation) _scale)))
      (bind _output_get_3 (Variables|Default|SetPhysConstraint _returnvalue_4))
      (Transformation|AttachComponentToComponent _returnvalue_4 (Variables|Default|GetSkeletalMesh) "upperarm_r" "SnapToTarget" "KeepWorld" "KeepWorld" true)
      (Class|PhysicsConstraintComponent|SetConstrainedComponents _output_get_3 (Variables|Default|GetSkeletalMesh) "upperarm_r" (Variables|/Script/Engine.StaticMeshActor|GetStaticMeshComponent (Variables|Default|GetMyMeshSpawned)) "None")
      (Class|PhysicsConstraintComponent|SetAngularSwing1Limit (Variables|Default|GetPhysConstraint) "ACM_Locked" 0.0)
      (Class|PhysicsConstraintComponent|SetAngularSwing2Limit (Variables|Default|GetPhysConstraint) "ACM_Locked" 0.0)
      (Class|PhysicsConstraintComponent|SetLinearXLimit (Variables|Default|GetPhysConstraint) "LCM_Limited" 5.0)
      (Class|PhysicsConstraintComponent|SetLinearZLimit (Variables|Default|GetPhysConstraint) "LCM_Limited" (Variables|Default|GetLimit%20Size))
      (Class|PhysicsConstraintComponent|SetAngularTwistLimit (Variables|Default|GetPhysConstraint) "ACM_Limited" 4e+01))))

(fn ConstructionScript)