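; Test actor for breaking a bone off a physics-driven skeletal component.
; BeginPlay and OnBoneBreak share one path that unhides the named bone on BonePhysicActor and breaks its constraint with zero impulse.
; Disconnected leftover logic hides all bones, spawns a simulated mannequin head mesh, and tethers it at the right upper-arm socket with a cable and limited physics constraint; none of it runs.
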(event Custom|OnBoneBreak
  (bind _bonename (Variables|Default|GetBoneName))
  (Components|SkinnedMesh|UnHideBonebyName (Variables|Default|GetBonePhysicActor) _bonename)
  (Class|SkeletalMeshComponent|BreakConstraint (Variables|Default|GetBonePhysicActor) "0, 0, 0" "0, 0, 0" _bonename))

(event EventBeginPlay
  (bind _bonename (Variables|Default|GetBoneName))
  (Components|SkinnedMesh|UnHideBonebyName (Variables|Default|GetBonePhysicActor) _bonename)
  (Class|SkeletalMeshComponent|BreakConstraint (Variables|Default|GetBonePhysicActor) "0, 0, 0" "0, 0, 0" _bonename))

(fn ConstructionScript)